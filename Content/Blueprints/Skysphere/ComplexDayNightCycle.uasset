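; Day-night cycle Blueprint that moves a sun light by latitude and time of year and updates the sky sphere.
; Tick advances the clock and day count, then SunTrajectory derives declination from a yearly cosine.
; Pitch follows piecewise parabolas over night and day, sized by the sunrise hour-angle formula or fixed quarter-days when polar, while yaw turns linearly.
; Polar and equator-flip flags refresh at BeginPlay and each day rollover.
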(event EventBeginPlay
  (Variables|Default|SetSunDeclanation (* (Math|Trig|Cos(Radians) (Math|Float|MultiplybyPi (* (/ (+ (/ (Variables|Default|GetClockWork) 24.0) (Math|Conversions|ToFloat(Integer) (Variables|Default|GetIntSunDays))) (Variables|Default|GetSunYearDuration)) 2.0))) (Variables|Default|GetMaxDeclanation)))
  (if (> (+ (- 9e+01 (Variables|Default|GetLatitude)) (Variables|Default|GetSunDeclanation)) 9e+01)
    (Variables|Default|SetEquatorFlip -1.0)
    (else
      (Variables|Default|SetEquatorFlip 1.0)))
  (if (or (< (- 9e+01 (+ (Variables|Default|GetLatitude) (Variables|Default|GetSunDeclanation))) 0.0) (< (- 9e+01 (- (Variables|Default|GetLatitude) (Variables|Default|GetSunDeclanation))) 0.0))
    (Variables|Default|SetPolar? true)
    (else
      (Variables|Default|SetPolar? false))))

(event EventTick
  (params (DeltaSeconds :type Float%20%28single-precision%29))
  (bind _timeunit (Variables|Default|GetTimeUnit))
  (bind _returnvalue (/ DeltaSeconds _timeunit))
  (Variables|Default|SetSunDrive (+ _returnvalue (Variables|Default|GetSunDrive)))
  (Variables|Default|SetClockWork (.Remainder (Math|Float|Division(WholeandRemainder) (+ (* (/ _returnvalue (Variables|Default|GetSunDayDuration)) 24.0) (Variables|Default|GetClockWork)) 24.0)))
  (Variables|Default|SetIntSunDays (Math|Float|Floor (.Remainder (Math|Float|Division(WholeandRemainder) (Math|Conversions|ToFloat(Integer) (+ (.ReturnValue (Math|Float|Division(WholeandRemainder) (+ (* (/ _returnvalue (Variables|Default|GetSunDayDuration)) 24.0) (Variables|Default|GetClockWork)) 24.0)) (Variables|Default|GetIntSunDays))) (Variables|Default|GetSunYearDuration)))))
  (CallFunction|SunTrajectory)
  (Transformation|SetActorRotation (Variables|Default|GetSunLight) (Math|Rotator|MakeRotator (Variables|Default|GetSunPitch) (Variables|Default|GetSunYaw) 0.0))
  (Default|UpdateSunDirection (Variables|Default|GetBP_Sky_Sphere))
  (if (>= (Variables|Default|GetSunDrive) (Variables|Default|GetSunDayDuration))
    (Variables|Default|SetSunDrive 0.0)
    (if (> (+ (- 9e+01 (Variables|Default|GetLatitude)) (Variables|Default|GetSunDeclanation)) 9e+01)
      (Variables|Default|SetEquatorFlip -1.0)
      (else
        (Variables|Default|SetEquatorFlip 1.0)))
    (if (or (< (- 9e+01 (+ (Variables|Default|GetLatitude) (Variables|Default|GetSunDeclanation))) 0.0) (< (- 9e+01 (- (Variables|Default|GetLatitude) (Variables|Default|GetSunDeclanation))) 0.0))
      (Variables|Default|SetPolar? true)
      (else
        (Variables|Default|SetPolar? false)))))

(fn ConstructionScript)

(fn SunTrajectory
  (bind _sundayduration (Variables|Default|GetSunDayDuration))
  (bind _returnvalue (* _sundayduration 0.25))
  (bind _returnvalue_2 (* _sundayduration 0.75))
  (Variables|Default|SetSunDeclanation (* (Math|Trig|Cos(Radians) (Math|Float|MultiplybyPi (* (/ (+ (/ (Variables|Default|GetClockWork) 24.0) (Math|Conversions|ToFloat(Integer) (Variables|Default|GetIntSunDays))) (Variables|Default|GetSunYearDuration)) 2.0))) (Variables|Default|GetMaxDeclanation)))
  (if (Variables|Default|GetPolar?)
    (if (<= (Variables|Default|GetSunDrive) _returnvalue)
      (Variables|Default|SetDayNightFlip -1.0)
      (Variables|Default|SetShift 0.0)
      (Variables|Default|SetSunPitch (- (* (Math|Float|Square (* (/ (- (Variables|Default|GetSunDrive) (Variables|Default|GetShift)) (* (Variables|Default|GetSunDayDuration) 0.25)) (Math|Float|Sqrt (- 9e+01 (Math|Float|Absolute(Float) (Variables|Default|GetLatitude)))))) (Variables|Default|GetDayNightFlip)) (* (Variables|Default|GetDayNightFlip) (- 9e+01 (- (Variables|Default|GetLatitude) (* (Variables|Default|GetSunDeclanation) (Variables|Default|GetDayNightFlip)))))) :!label _label)
      (Variables|Default|SetSunYaw (+ (* (/ (* (Variables|Default|GetSunDrive) 3.6e+02) (Variables|Default|GetSunDayDuration)) (Variables|Default|GetEquatorFlip)) (* (- 1.0 (Variables|Default|GetEquatorFlip)) 9e+01)) :!label _label_2)
      (elif (and (> (Variables|Default|GetSunDrive) _returnvalue) (<= (Variables|Default|GetSunDrive) _returnvalue_2))
        (Variables|Default|SetDayNightFlip 1.0)
        (Variables|Default|SetShift (/ (Variables|Default|GetSunDayDuration) 2.0))
        (goto _label)
        (elif (> (Variables|Default|GetSunDrive) _returnvalue_2)
          (Variables|Default|SetDayNightFlip -1.0)
          (Variables|Default|SetShift (Variables|Default|GetSunDayDuration))
          (goto _label))))
    (else
      (Variables|Default|SetSunHalfDayLight (/ (Math|Trig|Acos(Degrees) (* (Math|Trig|Tan(Degrees) (Variables|Default|GetLatitude)) (Math|Trig|Tan(Degrees) (* (Variables|Default|GetSunDeclanation) -1.0)))) (/ (Math|Trig|DegreesToRadians 3.6e+02) (Variables|Default|GetSunDayDuration))))
      (Variables|Default|SetSunHalfNight (/ (Math|Trig|Acos(Degrees) (* (Math|Trig|Tan(Degrees) (Variables|Default|GetLatitude)) (Math|Trig|Tan(Degrees) (Variables|Default|GetSunDeclanation)))) (/ (Math|Trig|DegreesToRadians 3.6e+02) (Variables|Default|GetSunDayDuration))))
      (if (<= (Variables|Default|GetSunDrive) (Variables|Default|GetSunHalfNight))
        (Variables|Default|SetDayNightFlip -1.0)
        (Variables|Default|SetShift 0.0)
        (Variables|Default|SetLength (Variables|Default|GetSunHalfNight))
        (Variables|Default|SetSunPitch (- (* (Math|Float|Square (* (/ (- (Variables|Default|GetSunDrive) (Variables|Default|GetShift)) (Variables|Default|GetLength)) (Math|Float|Sqrt (- 9e+01 (Math|Float|Absolute(Float) (- (Variables|Default|GetLatitude) (* (Variables|Default|GetSunDeclanation) (Variables|Default|GetDayNightFlip)))))))) (Variables|Default|GetDayNightFlip)) (* (Variables|Default|GetDayNightFlip) (- 9e+01 (Math|Float|Absolute(Float) (- (Variables|Default|GetLatitude) (* (Variables|Default|GetSunDeclanation) (Variables|Default|GetDayNightFlip))))))) :!label _label_3)
        (goto _label_2)
        (elif (and (> (Variables|Default|GetSunDrive) (Variables|Default|GetSunHalfNight)) (<= (Variables|Default|GetSunDrive) (+ (Variables|Default|GetSunHalfNight) (* (Variables|Default|GetSunHalfDayLight) 2.0))))
          (Variables|Default|SetDayNightFlip 1.0)
          (Variables|Default|SetShift (/ (Variables|Default|GetSunDayDuration) 2.0))
          (Variables|Default|SetLength (Variables|Default|GetSunHalfDayLight))
          (goto _label_3)
          (elif (> (Variables|Default|GetSunDrive) (+ (Variables|Default|GetSunHalfNight) (* (Variables|Default|GetSunHalfDayLight) 2.0)))
            (Variables|Default|SetDayNightFlip -1.0)
            (Variables|Default|SetShift (Variables|Default|GetSunDayDuration))
            (Variables|Default|SetLength (Variables|Default|GetSunHalfNight))
            (goto _label_3)))))))